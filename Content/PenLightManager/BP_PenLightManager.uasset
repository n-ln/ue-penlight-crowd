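; BP_PenLightManager adds debug keyboard controls for the pen lights' waving, on/off state, color and intensity.
; BeginPlay enables input from player controller 0, and debug keys call the manager's getters and setters, which are not defined in this graph.
; Keys toggle waving and lights, step intensity with a floor at zero, and rotate hue in HSV space with fixed saturation and value.
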(event EventBeginPlay
  (Input|EnableInput (Game|GetPlayerController 0)))

(event EventTick
  (params (DeltaSeconds :type Float%20%28single-precision%29)))

(event Input|KeyboardEvents|DebugKeyP
  (params (Key :type Key%20Structure :default "None") (ActionValue :type Input%20Action%20Value%20Structure))
  (:Pressed
    (Class|PenLightManager|SetLightson (not (Class|PenLightManager|GetLightson)))))

(event Input|KeyboardEvents|DebugKeyI
  (params (Key :type Key%20Structure :default "None") (ActionValue :type Input%20Action%20Value%20Structure))
  (:Pressed
    (Class|PenLightManager|SetPenLightIntensity (Math|Float|Max(Float) (- (Class|PenLightManager|GetPenLightIntensity) 1e+01) 0.0))))

(event Input|KeyboardEvents|DebugKeyO
  (params (Key :type Key%20Structure :default "None") (ActionValue :type Input%20Action%20Value%20Structure))
  (:Pressed
    (Class|PenLightManager|SetPenLightIntensity (+ (Class|PenLightManager|GetPenLightIntensity) 1e+01))))

(event Input|KeyboardEvents|DebugKeyM
  (params (Key :type Key%20Structure :default "None") (ActionValue :type Input%20Action%20Value%20Structure))
  (:Pressed
    (Class|PenLightManager|SetIsWaving (not (Class|PenLightManager|GetIsWaving)))))

(event Input|KeyboardEvents|DebugKeyK
  (params (Key :type Key%20Structure :default "None") (ActionValue :type Input%20Action%20Value%20Structure))
  (:Pressed
    (Class|PenLightManager|SetPenLightColor (Class|KismetMathLibrary|HSVtoRGBLinear (Utilities|Struct|MakeLinearColor (Math|Float|%(Float) (+ (.r (Class|KismetMathLibrary|RGBLineartoHSV (Class|PenLightManager|GetPenLightColor))) 3e+01) 3.6e+02) 0.8 1.0 1.0)))))

(event Input|KeyboardEvents|DebugKeyL
  (params (Key :type Key%20Structure :default "None") (ActionValue :type Input%20Action%20Value%20Structure))
  (:Pressed
    (Class|PenLightManager|SetPenLightColor (Class|KismetMathLibrary|HSVtoRGBLinear (Utilities|Struct|MakeLinearColor (Math|Float|%(Float) (+ (.r (Class|KismetMathLibrary|RGBLineartoHSV (Class|PenLightManager|GetPenLightColor))) -3e+01) 3.6e+02) 0.8 1.0 1.0)))))

(fn ConstructionScript)